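; Enemy NPC that shoots projectiles and handles its own death.
; FireBullet spawns an EnemyProjectile and sound at the barrel arrow, provided its AI controller has a valid focus actor.
; When its health system component reports a kill, it plays death sound and particles, then destroys itself.
; Before destruction, it uses the AI_NPC controller's game mode reference to fade combat music back to ambient and clear the combat flag.
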(event OnKilled(BP_HealthSystemComponent)
  (bind _returnvalue (Transformation|GetActorLocation))
  (Audio|PlaySoundatLocation "/Game/_Game/Audio/enemyDeath_Cue.enemyDeath_Cue" _returnvalue "0, 0, 0" 1.0 1.0 0.0 0 0 0 0)
  (Niagara|SpawnSystematLocation "/Game/_Game/Particles/PlayerDeathBurst.PlayerDeathBurst" _returnvalue)
  (Utilities|FlowControl|Sequence
    (:then_0
      (bind _asai_npc (Utilities|Casting|CastToAI_NPC (AI|GetAIController self)))
      (if (Variables|/Game/FirstPerson/Blueprints/BP_FirstPersonGameMode.BP_FirstPersonGameMode_C|GetCombatMusicPlaying? (Variables|/Game/_Game/AI/AI_NPC.AI_NPC_C|GetGame%20Mode%20REF _asai_npc))
        (Class|BPIMusicPlayer|PlayMusic(Message) (Game|GetGameInstance) "/Game/_Game/Audio/Music/ambient_track_Cue.ambient_track_Cue" 3.0 3.0)
        (Variables|/Game/FirstPerson/Blueprints/BP_FirstPersonGameMode.BP_FirstPersonGameMode_C|SetCombatMusicPlaying? (Variables|/Game/_Game/AI/AI_NPC.AI_NPC_C|GetGame%20Mode%20REF _asai_npc) false)))
    (:then_1
      (Actor|DestroyActor))))

(event Custom|FireBullet
  (bind _barrel_arrow (Variables|Default|GetBarrel%20Arrow))
  (bind _returnvalue (Transformation|GetWorldLocation _barrel_arrow))
  (Utilities|IsValid (Class|AIController|GetFocusActor (AI|GetAIController self))
    (:Is%20Valid
      (Game|SpawnActorfromClass "/Game/_Game/AI/EnemyProjectile.EnemyProjectile_C" (Math|Transform|MakeTransform _returnvalue (Transformation|GetWorldRotation _barrel_arrow) "1.000000,1.000000,1.000000") "Undefined" "MultiplyWithRoot" 0 0)
      (Audio|PlaySoundatLocation "/Game/FirstPerson/Audio/Cues/DamageSound.DamageSound" _returnvalue "0, 0, 0" 1.0 1.0 0.0 0 0 0 0))
    (:Is%20Not%20Valid
      (Development|PrintString "Bullet Firing Not Valid"))))

(fn ConstructionScript)