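; Pressure plate switch actor that turns on while overlapped and off when an overlap ends, with no filter on which actor triggers it.
; The SwitchActivate timeline moves the Switch component's height, playing on begin overlap and reversing on end overlap.
; SwitchActivated becomes true only when forward playback finishes, guarded by the Reversed flag, but clears immediately on release.
; Each state change prints the value and plays an attenuated on or off sound.
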(event Collision|EventActorBeginOverlap
  (params (OtherActor :type Actor%20Object%20Reference))
  (Variables|Default|SetReversed? false)
  (bind _switchposition (Timeline|SwitchActivate Play)
    (:Update
      (Transformation|SetRelativeLocation (Variables|Default|GetSwitch) (Math|Vector|MakeVector 0.0 0.0 _switchposition) false false))
    (:Finished
      (if (not (Variables|Default|GetReversed?))
        (bind _output_get (Variables|Default|SetSwitchActivated? true))
        (Development|PrintString (Utilities|String|ToString(Boolean) _output_get))
        (Audio|PlaySoundatLocation "/Game/_Game/Audio/plate_on_Cue.plate_on_Cue" (Transformation|GetActorLocation) "0, 0, 0" 1.0 1.0 0.0 "/Game/_Game/Audio/Attenuation/SA_PressurePlate.SA_PressurePlate" 0 0 0)))))

(event Collision|EventActorEndOverlap
  (params (OtherActor :type Actor%20Object%20Reference))
  (bind _returnvalue (Transformation|GetActorLocation))
  (bind _output_get (Variables|Default|SetSwitchActivated? false))
  (Development|PrintString (Utilities|String|ToString(Boolean) _output_get))
  (Audio|PlaySoundatLocation "/Game/_Game/Audio/plate_off_Cue.plate_off_Cue" _returnvalue "0, 0, 0" 1.0 1.0 0.0 "/Game/_Game/Audio/Attenuation/SA_PressurePlate.SA_PressurePlate" 0 0 0)
  (Variables|Default|SetReversed? true)
  (bind _switchposition (Timeline|SwitchActivate Reverse)
    (:Update
      (Transformation|SetRelativeLocation (Variables|Default|GetSwitch) (Math|Vector|MakeVector 0.0 0.0 _switchposition) false false))
    (:Finished
      (if (not (Variables|Default|GetReversed?))
        (bind _output_get_2 (Variables|Default|SetSwitchActivated? true))
        (Development|PrintString (Utilities|String|ToString(Boolean) _output_get_2))
        (Audio|PlaySoundatLocation "/Game/_Game/Audio/plate_on_Cue.plate_on_Cue" _returnvalue "0, 0, 0" 1.0 1.0 0.0 "/Game/_Game/Audio/Attenuation/SA_PressurePlate.SA_PressurePlate" 0 0 0)))))

(fn ConstructionScript)