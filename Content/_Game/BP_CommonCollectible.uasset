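; BP_CommonCollectible is a pickup actor that adds to the player's common collectible count when touched.
; Its Box overlap responds only to player character 0, playing a coin sound and spawning a burst effect at its location.
; It then adds CollectibleValue to CommonCollectibleCount on BP_FirstPersonPlayerController and destroys itself.
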(event OnComponentBeginOverlap(Box)
  (params (OverlappedComponent :type Primitive%20Component%20Object%20Reference) (OtherActor :type Actor%20Object%20Reference) (OtherComp :type Primitive%20Component%20Object%20Reference) (OtherBodyIndex :type Integer) (bFromSweep :type Boolean) (SweepResult :type Hit%20Result%20Structure%20%28by%20ref%29))
  (bind _returnvalue (Transformation|GetActorLocation))
  (if (== OtherActor (Game|GetPlayerCharacter 0))
    (Audio|PlaySoundatLocation "/Game/_Game/Audio/coin_Cue.coin_Cue" _returnvalue "0, 0, 0" 1.0 1.0 0.0 0 0 0 0)
    (Niagara|SpawnSystematLocation "/Game/_Game/Particles/CollectibleBurst.CollectibleBurst" _returnvalue)
    (bind _asbp_first_person_player_controller (Utilities|Casting|CastToBP_FirstPersonPlayerController (Game|GetPlayerController 0)))
    (Variables|/Game/FirstPerson/Blueprints/BP_FirstPersonPlayerController.BP_FirstPersonPlayerController_C|SetCommonCollectibleCount _asbp_first_person_player_controller (+ (Variables|Default|GetCollectibleValue) (Variables|/Game/FirstPerson/Blueprints/BP_FirstPersonPlayerController.BP_FirstPersonPlayerController_C|GetCommonCollectibleCount _asbp_first_person_player_controller)))
    (Actor|DestroyActor)))

(fn ConstructionScript)