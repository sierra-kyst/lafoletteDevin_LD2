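; BP_Laser is a humming laser hazard that slides along a random path and burns actors that touch it.
; The construction script randomly picks a movement behavior, and BeginPlay sets a random distance along local Y or Z.
; The LaserMovement timeline lerps the Cylinder's relative location to that point.
; Box overlap applies damage with a burn sound, repeating through a Delay loop until overlap ends.
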(event OnComponentBeginOverlap(Box)
  (params (OverlappedComponent :type Primitive%20Component%20Object%20Reference) (OtherActor :type Actor%20Object%20Reference) (OtherComp :type Primitive%20Component%20Object%20Reference) (OtherBodyIndex :type Integer) (bFromSweep :type Boolean) (SweepResult :type Hit%20Result%20Structure%20%28by%20ref%29))
  (Variables|Default|SetIsOverlapping? true)
  (Game|Damage|ApplyDamage OtherActor 5.0 0 self :!label _label)
  (Audio|PlaySoundatLocation "/Game/_Game/Audio/burned_01_Cue.burned_01_Cue" (Transformation|GetActorLocation) "0, 0, 0" 1.0 1.0 0.0 0 0 0 0)
  (Utilities|FlowControl|Delay 0.5)
  (if (Variables|Default|GetIsOverlapping?)
    (goto _label)))

(event OnComponentEndOverlap(Box)
  (params (OverlappedComponent :type Primitive%20Component%20Object%20Reference) (OtherActor :type Actor%20Object%20Reference) (OtherComp :type Primitive%20Component%20Object%20Reference) (OtherBodyIndex :type Integer))
  (Variables|Default|SetIsOverlapping? false))

(event EventBeginPlay
  (bind _returnvalue (Math|Random|RandomFloatinRange 1e+02 3.5e+02))
  (Audio|PlaySoundatLocation "/Game/_Game/Audio/laser_hum_Cue.laser_hum_Cue" (Transformation|GetActorLocation) "0, 0, 0" 1.0 1.0 0.0 "/Game/_Game/Audio/Attenuation/SA_LaserHum.SA_LaserHum" 0 0 0)
  (switch Utilities|FlowControl|Switch|SwitchonE_LaserBehavior (Variables|Default|GetLaserBehavior)
    (:NewEnumerator1
      (Variables|Default|SetDestinationLocation (Math|Vector|MakeVector 0.0 _returnvalue 0.0))
      (bind _alpha (Timeline|Laser%20Movement Play)
        (:Update
          (switch Utilities|FlowControl|Switch|SwitchonE_LaserBehavior (Variables|Default|GetLaserBehavior)
            (:NewEnumerator1
              _)
            (:NewEnumerator2
              _))
          (Transformation|SetRelativeLocation (Variables|Default|GetCylinder) (Math|Vector|Lerp(Vector) "0, 0, 0" (Variables|Default|GetDestinationLocation) _alpha) false false))))
    (:NewEnumerator2
      (Variables|Default|SetDestinationLocation (Math|Vector|MakeVector 0.0 0.0 _returnvalue))
      (Timeline|Laser%20Movement Play))))

(fn ConstructionScript
  (Variables|Default|SetLaserBehavior (Utilities|Enum|ByteToEnumE_LaserBehavior (Math|Conversions|ToByte(Integer) (Math|Random|RandomIntegerinRange 1 2)))))