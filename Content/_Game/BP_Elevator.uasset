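; BP_Elevator is an elevator that descends once, triggered when the player enters it or its trigger box.
; The Box overlap passes through a DoOnce, prints a debug message and plays a ding-dong cue at the back wall's relative location.
; The ElevatorGoesDown timeline then drives the Floor component's relative Z directly from its Alpha track, with no return trip.
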(event OnComponentBeginOverlap(Box)
  (params (OverlappedComponent :type Primitive%20Component%20Object%20Reference) (OtherActor :type Actor%20Object%20Reference) (OtherComp :type Primitive%20Component%20Object%20Reference) (OtherBodyIndex :type Integer) (bFromSweep :type Boolean) (SweepResult :type Hit%20Result%20Structure%20%28by%20ref%29))
  (if (== OtherActor (Game|GetPlayerCharacter 0))
    (Utilities|FlowControl|DoOnce false
      (:Completed
        (Development|PrintString "Going down!")
        (Audio|PlaySoundatLocation "/Game/_Game/Audio/dingdong_Cue.dingdong_Cue" (Variables|/Script/Engine.SceneComponent|GetRelativeLocation (Variables|Default|GetWallBack)) "0, 0, 0" 1.0 1.0 0.0 0 0 0 0)
        (bind _alpha (Timeline|Elevator%20goes%20down PlayFromStart)
          (:Update
            (Transformation|SetRelativeLocation (Variables|Default|GetFloor) (Math|Vector|MakeVector 0.0 0.0 _alpha) false false)))))))

(fn ConstructionScript)