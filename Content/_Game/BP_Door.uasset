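; BP_Door is a sliding door actor that raises and lowers its Cube mesh with open and close sounds.
; Tick polls the DoorOpened flag, and a pair of DoOnce nodes, each reset by the opposite state, fires each transition once.
; The DoorOpen timeline plays or reverses to lerp the cube's relative Z, while spatialized sound cues play at the actor's location.
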(event EventTick
  (params (DeltaSeconds :type Float%20%28single-precision%29))
  (bind _returnvalue (Transformation|GetActorLocation))
  (bind _dooropened_ (Variables|Default|GetDoorOpened?))
  (Utilities|FlowControl|Sequence
    (:then_0
      (if _dooropened_
        (Utilities|FlowControl|DoOnce false :!label _label
          (:Completed
            (Audio|PlaySoundatLocation "/Game/_Game/Audio/door_opened_Cue.door_opened_Cue" _returnvalue "0, 0, 0" 1.0 1.0 0.0 "/Game/_Game/Audio/Attenuation/SA_DoorAmbi.SA_DoorAmbi" 0 0 0)
            (bind _alpha (Timeline|Door%20Open Play)
              (:Update
                (Transformation|SetRelativeLocation (Variables|Default|GetCube) (Math|Vector|MakeVector 0.0 0.0 (Math|Float|Lerp 1.5e+02 4.5e+02 _alpha)) false false)))))
        (else
          (Utilities|FlowControl|DoOnce true :!label _label_2
            (:Completed
              (Audio|PlaySoundatLocation "/Game/_Game/Audio/door_closed_Cue.door_closed_Cue" _returnvalue "0, 0, 0" 1.0 1.0 0.0 "/Game/_Game/Audio/Attenuation/SA_DoorAmbi.SA_DoorAmbi" 0 0 0)
              (Timeline|Door%20Open Reverse))))))
    (:then_1
      (if _dooropened_
        (goto _label_2 Reset)
        (else
          (goto _label Reset))))))

(fn ConstructionScript)