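; BP_BoltProjectile is a bouncing electric bolt projectile with a looping-style ambient sound attached to its sphere.
; On bounce, it damages actors implementing ZappableByBolt and destroys itself with an impact sound and effect; other surfaces only play a bounce sound.
; A five-second timer from BeginPlay otherwise detonates it, applying small-radius, full-strength radial damage before destroying it.
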(event OnProjectileBounce(ProjectileMovement)
  (params (ImpactResult :type Hit%20Result%20Structure%20%28by%20ref%29) (ImpactVelocity :type Vector%20%28by%20ref%29 :default "0, 0, 0"))
  (bind _hitactor (Collision|BreakHitResult ImpactResult))
  (bind _returnvalue (Transformation|GetActorLocation))
  (if (Utilities|DoesObjectImplementInterface _hitactor "/Game/_Game/ZappableByBolt.ZappableByBolt_C")
    (Audio|PlaySoundatLocation "/Game/_Game/Audio/ZapImpact_Cue.ZapImpact_Cue" _returnvalue "0, 0, 0" 1.0 1.0 0.0 "/Game/_Game/Audio/Attenuation/SA_BoltAmbi.SA_BoltAmbi" 0 0 0)
    (Niagara|SpawnSystematLocation 0 _returnvalue)
    (Game|Damage|ApplyDamage _hitactor 1e+02 0 0)
    (Variables|Default|SetActiveBolt? false)
    (Actor|DestroyActor)
    (else
      (Audio|PlaySoundatLocation "/Game/_Game/Audio/boltBounce_Cue.boltBounce_Cue" _returnvalue "0, 0, 0" 1.0 1.0 0.0 "/Game/_Game/Audio/Attenuation/SA_BoltAmbi.SA_BoltAmbi" 0 0 0))))

(event Custom|DelayAction
  (bind _returnvalue (Transformation|GetActorLocation))
  (Audio|PlaySoundatLocation "/Game/_Game/Audio/ZapImpact_Cue.ZapImpact_Cue" _returnvalue "0, 0, 0" 1.0 1.0 0.0 "/Game/_Game/Audio/Attenuation/SA_BoltAmbi.SA_BoltAmbi" 0 0 0)
  (Niagara|SpawnSystematLocation 0 _returnvalue)
  (Game|Damage|ApplyRadialDamage 1e+02 _returnvalue 6e+01 0 0 0 0 true "ECC_Visibility")
  (Variables|Default|SetActiveBolt? false)
  (Actor|DestroyActor))

(event EventBeginPlay
  (bind _sphere (Variables|Default|GetSphere))
  (Audio|SpawnSoundAttached "/Game/_Game/Audio/electricAmbi_Cue.electricAmbi_Cue" _sphere "None" (Variables|/Script/Engine.SceneComponent|GetRelativeLocation _sphere) "0, 0, 0" "KeepRelativeOffset" true 1.0 1.0 0.0 "/Game/_Game/Audio/Attenuation/SA_BoltAmbi.SA_BoltAmbi" 0)
  (Utilities|Time|SetTimerbyEvent (delegate Custom|DelayAction) 5.0))

(fn ConstructionScript)