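; BP_BeaconAntenna is a beacon antenna actor that activates when it takes damage.
; On BeginPlay it creates a dynamic material instance on the BeaconBulb and binds to its any-damage event.
; DamageFlash sets the bulb's emissive color and intensity with no reset, then a DoOnce plays a puzzle cue at the actor and sets BeaconIsActivated.
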(event Custom|DamageFlash
  (params (DamagedActor :type Actor%20Object%20Reference) (Damage :type Float%20%28single-precision%29) (DamageType :type Damage%20Type%20Object%20Reference) (InstigatedBy :type Controller%20Object%20Reference) (DamageCauser :type Actor%20Object%20Reference))
  (bind _flashmat (Variables|Default|GetFlashMat))
  (Rendering|Material|SetVectorParameterValue _flashmat "EmissiveColor" (Variables|Default|GetFlashColor) :!class /Script/Engine.MaterialInstanceDynamic)
  (Rendering|Material|SetScalarParameterValue _flashmat "EmissiveMultiplier" (Variables|Default|GetFlashIntensity) :!class /Script/Engine.MaterialInstanceDynamic)
  (Utilities|FlowControl|DoOnce false
    (:Completed
      (Audio|PlaySoundatLocation "/Game/_Game/Audio/Puzzle_Cue.Puzzle_Cue" (Transformation|GetActorLocation) "0, 0, 0" 1.0 1.0 0.0 0 0 0 0)
      (Variables|Default|SetBeaconIsActivated? true))))

(event EventBeginPlay
  ;[1 1 1] Setup Dynamic Material Instance from Actor
  (EventDispatchers|BindEventtoOnTakeAnyDamage (EventDispatchers|CreateEvent :!event Custom|DamageFlash))
  (bind _returnvalue (Rendering|Material|CreateDynamicMaterialInstance (Variables|Default|GetBeaconBulb) 0 0 "None" :!class /Script/Engine.PrimitiveComponent))
  (Variables|Default|SetFlashMat _returnvalue))

(fn ConstructionScript)